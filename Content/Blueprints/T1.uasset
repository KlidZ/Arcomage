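; T1 is a Blueprint with a Cylinder component and a Turn event that acts according to an Index value.
; Turn switches on Index, printing debug numbers for two cases and nudging the Cylinder upward in world space for another.
; An unconnected lookup of DataBase actors and their PickedCard value never runs, and the construction script is empty.
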(event `Turn`
  (bind _cylinder (`self.Cylinder`))
  (bind (_returnvalue_x _returnvalue_y _returnvalue_z) (`KismetMathLibrary.BreakVector` (`SceneComponent.K2_GetComponentLocation` _cylinder)))
  (switch `int` (`self.Index`)
    (:`2`
      (`KismetSystemLibrary.PrintString` "2"))
    (:`4`
      (`KismetSystemLibrary.PrintString` "4"))
    (:`5`
      (`SceneComponent.K2_SetWorldLocation` _cylinder (`KismetMathLibrary.MakeVector` _returnvalue_x _returnvalue_y (+ _returnvalue_z 15.0)) false false))))

(fn `UserConstructionScript`)